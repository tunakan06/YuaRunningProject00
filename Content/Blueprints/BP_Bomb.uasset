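; BP_Bomb is a moving hazard that explodes on overlap and damages the player.
; Tick oscillates it along world X by adding a sine-of-game-time offset each frame, so travel depends on frame rate.
; Any Sphere overlap spawns a Niagara effect, then subtracts Health from player 0's BP_ThirdPersonCharacter without checking the overlapping actor.
; The bomb then destroys itself, and destroys the character if Health drops below zero.
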(event `self.ReceiveTick`
  (params (DeltaSeconds :type "Float (single-precision)"))
  (bind (_returnvalue_x _returnvalue_y _returnvalue_z) (`KismetMathLibrary.BreakVector` (`self.K2_GetActorLocation`)))
  (`self.K2_SetActorLocation` (`KismetMathLibrary.MakeVector` (+ _returnvalue_x (* (`KismetMathLibrary.Sin` (`KismetSystemLibrary.GetGameTimeInSeconds`)) 10.0)) _returnvalue_y _returnvalue_z)))

(event `self.Sphere.OnComponentBeginOverlap`
  (params (OverlappedComponent :type "PrimitiveComponent Object Reference") (OtherActor :type "Actor Object Reference") (OtherComp :type "PrimitiveComponent Object Reference") (OtherBodyIndex :type Integer) (bFromSweep :type Boolean) (SweepResult :type "HitResult Structure (by ref)"))
  (`NiagaraFunctionLibrary.SpawnSystemAtLocation` "/Game/sA_PickupSet_1/Fx/NiagaraSystems/NS_Energy_2.NS_Energy_2" (`self.K2_GetActorLocation`))
  (bind _asbp_third_person_character (cast `/Game/ThirdPerson/Blueprints/BP_ThirdPersonCharacter` (`GameplayStatics.GetPlayerCharacter` 0)))
  (bind _output_get (set `/Game/ThirdPerson/Blueprints/BP_ThirdPersonCharacter.Health` (- (`/Game/ThirdPerson/Blueprints/BP_ThirdPersonCharacter.Health` _asbp_third_person_character) 60.0) _asbp_third_person_character))
  (`self.K2_DestroyActor`)
  (if (< _output_get 0.0)
    (`self.K2_DestroyActor` _asbp_third_person_character)))

(fn `UserConstructionScript`)